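; HUD Blueprint for UBomber that owns the on-screen HUD widget and controls its end screen.
; On BeginPlay it creates the widget and adds it to the viewport only for the player controller with ID 0, keeping a reference to it.
; The show and close end-screen events forward to that widget when the reference is valid, with show passing along the display text.
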(event EventBeginPlay
  (bind _returnvalue (Game|Player|GetOwningPlayerController))
  ;[1 1 1] Prepare HUD
  (bind _returnvalue_2 (Class|GameplayStatics|GetPlayerControllerID _returnvalue))
  (if (== _returnvalue_2 0)
    (bind _returnvalue_3 (UserInterface|CreateWidget "/Game/Blueprints/UI/HUDWidget.HUDWidget_C" _returnvalue))
    (Variables|Default|SetHUDWidgetReference _returnvalue_3)
    (UserInterface|Viewport|AddtoViewport _returnvalue_3 0)))

(event EventCloseEndScreenBPEvent
  ;[1 1 1] Hide end screen
  (Utilities|IsValid (Variables|Default|GetHUDWidgetReference)
    (:Is%20Valid
      (Default|HideEndScreen (Variables|Default|GetHUDWidgetReference)))))

(event EventShowEndScreenBPEvent
  (params (Text :type String))
  ;[1 1 1] Show end screen
  (Utilities|IsValid (Variables|Default|GetHUDWidgetReference)
    (:Is%20Valid
      (Default|ShowEndScreen (Variables|Default|GetHUDWidgetReference) Text))))

(fn ConstructionScript)