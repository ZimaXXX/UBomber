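; Bomber character Blueprint that adds a player name display and a damage debug readout on top of its parent class.
; When the player state is ready, it passes the player's name to the widget object held by its PlayerNameWidget component.
; Any damage received is only printed as a string; BeginPlay and Tick just call the parent, and the construction script is empty.
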(event EventBeginPlay
  (|CallParentFunction))

(event Collision|EventActorBeginOverlap
  (params (OtherActor :type Actor%20Object%20Reference)))

(event EventTick
  (params (DeltaSeconds :type Float%20%28single-precision%29))
  (|CallParentFunction DeltaSeconds))

(event EventPlayerStateReady
  ;[1 1 1] Set Player Name on Widget
  (|CallParentFunction)
  (bind _asplayer_name_widget (Utilities|Casting|CastToPlayerNameWidget (UserInterface|GetUserWidgetObject (Variables|Default|GetPlayerNameWidget))))
  (Default|SetPlayerName _asplayer_name_widget (Variables|/Script/Engine.PlayerState|GetPlayerName (Variables|Default|GetPlayerState self))))

(event Game|Damage|EventAnyDamage
  (params (Damage :type Float%20%28single-precision%29) (DamageType :type Damage%20Type%20Object%20Reference) (InstigatedBy :type Controller%20Object%20Reference) (DamageCauser :type Actor%20Object%20Reference))
  (Development|PrintString (Utilities|String|ToString(Float) Damage)))

(fn ConstructionScript)